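; BP_Key is a key pickup actor for a lock-and-key mechanic.
; On BeginPlay it caches the first player character as a BP_Player.
; When that player overlaps its sphere component, it sets the player's DoorKey flag to true and destroys itself.
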(event `self.ReceiveBeginPlay`
  (bind _asbp_player (cast `/Game/Blueprints/BP_Player` (`GameplayStatics.GetPlayerCharacter` 0)))
  (set `self.As BP Player` _asbp_player))

(event `PickUpKey`
  (set `/Game/Blueprints/BP_Player.DoorKey` true (`self.As BP Player`))
  (`self.K2_DestroyActor`))

(event `self.Sphere1.OnComponentBeginOverlap`
  (params (OverlappedComponent :type "PrimitiveComponent Object Reference") (OtherActor :type "Actor Object Reference") (OtherComp :type "PrimitiveComponent Object Reference") (OtherBodyIndex :type Integer) (bFromSweep :type Boolean) (SweepResult :type "HitResult Structure (by ref)"))
  (if (== OtherActor (`self.As BP Player`))
    (`self.PickUpKey`)))

(fn `UserConstructionScript`)